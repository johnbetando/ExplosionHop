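; GameInstance blueprint that holds the game's Master, Music and SFX volumes and persists them between sessions.
; Each setter applies a sound class override through its own sound mix, pushes that mix and caches the value.
; SaveVolumes writes the cached values to a new Volume_SaveGame in the "VolumeSave" slot, and SetVolumesFromSave loads that slot and reapplies them.
; GetVolumes returns the three current values to callers.
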(event `SetVolumesFromSave`
  (bind _returnvalue (`GameplayStatics.LoadGameFromSlot` "VolumeSave"))
  (bind _asvolume_save_game (cast `/Game/Blueprints/Volume_SaveGame` _returnvalue))
  (`self.SetMasterVolume` (`/Game/Blueprints/Volume_SaveGame.MasterVolume` _asvolume_save_game))
  (`self.SetMusicVolume` (`/Game/Blueprints/Volume_SaveGame.MusicVolume` _asvolume_save_game))
  (`self.SetSFXVolume` (`/Game/Blueprints/Volume_SaveGame.SFXVolume` _asvolume_save_game)))

(event `SaveVolumes`
  (bind _asgame_instance_bp (cast `/Game/Blueprints/GameInstance_BP` (`GameplayStatics.GetGameInstance`) :!pure true))
  (bind _returnvalue (`GameplayStatics.CreateSaveGameObject` "/Game/Blueprints/Volume_SaveGame.Volume_SaveGame_C"))
  (`/Game/Blueprints/Volume_SaveGame.SetSaveVolumes` _returnvalue (`/Game/Blueprints/GameInstance_BP.MasterVolume` _asgame_instance_bp) (`/Game/Blueprints/GameInstance_BP.MusicVolume` _asgame_instance_bp) (`/Game/Blueprints/GameInstance_BP.SFXVolume` _asgame_instance_bp))
  (`GameplayStatics.SaveGameToSlot` _returnvalue "VolumeSave"))

(event `SetMasterVolume`
  (params (Volume :type "Float (double-precision)"))
  (`GameplayStatics.SetSoundMixClassOverride` "/Game/Audio/MasterSoundMixClass.MasterSoundMixClass" "/Game/Audio/MasterSoundClass.MasterSoundClass" Volume 1.0 0.0)
  (`GameplayStatics.PushSoundMixModifier` "/Game/Audio/MasterSoundMixClass.MasterSoundMixClass")
  (set `self.MasterVolume` Volume))

(event `SetMusicVolume`
  (params (Volume :type "Float (double-precision)"))
  (`GameplayStatics.SetSoundMixClassOverride` "/Game/Audio/MusicSoundMixClass.MusicSoundMixClass" "/Game/Audio/MusicSoundClass.MusicSoundClass" Volume 1.0 0.0)
  (`GameplayStatics.PushSoundMixModifier` "/Game/Audio/MusicSoundMixClass.MusicSoundMixClass")
  (set `self.MusicVolume` Volume))

(event `SetSFXVolume`
  (params (Volume :type "Float (double-precision)"))
  (`GameplayStatics.SetSoundMixClassOverride` "/Game/Audio/SFXSoundMixClass.SFXSoundMixClass" "/Game/Audio/SFXSoundClass.SFXSoundClass" Volume 1.0 0.0)
  (`GameplayStatics.PushSoundMixModifier` "/Game/Audio/SFXSoundMixClass.SFXSoundMixClass")
  (set `self.SFXVolume` Volume))

(fn `GetVolumes`
  (returns (Master :type "Float (double-precision)") (Music :type "Float (double-precision)") (SFX :type "Float (double-precision)"))
  (return (`self.MasterVolume`) (`self.MusicVolume`) (`self.SFXVolume`)))