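; Barrel Blueprint that bobs its Cylinder component up and down.
; On BeginPlay, a looping two-second timer calls BobBarrel, with a random negative start delay to vary the phase between instances.
; Each call restarts BobbingTimeline, whose track value times BobbingSpeed sets the cylinder's relative Z, so BobbingSpeed scales bob height rather than rate.
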(event `self.ReceiveBeginPlay`
  (`parent.ReceiveBeginPlay`)
  (`KismetSystemLibrary.K2_SetTimer` null "BobBarrel" 2.0 true (`KismetMathLibrary.RandomFloatInRange` -2.0)))

(event `self.ReceiveTick`
  (params (DeltaSeconds :type "Float (single-precision)"))
  (`parent.ReceiveTick` DeltaSeconds))

(event `BobBarrel`
  (bind (_direction _newtrack_0) (`Timeline|BobbingTimeline` :!via `PlayFromStart`)
    (:`Update`
      (`SceneComponent.K2_SetRelativeLocation` (`self.Cylinder`) (`KismetMathLibrary.MakeVector` 0.0 0.0 (* _newtrack_0 (`self.BobbingSpeed`))) false false))))

(fn `UserConstructionScript`
  (`parent.UserConstructionScript`))