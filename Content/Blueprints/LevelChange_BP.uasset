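; LevelChange_BP is a trigger volume that moves the player to another level.
; On BeginPlay it caches the FirstPersonCharacter.
; When that character overlaps the Box component, it disables input, calls the character's FadeOut, waits briefly, then opens the level named in the LevelName variable.
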(event `self.ReceiveBeginPlay`
  (bind _asfirst_person_character (cast `/Game/FirstPersonBP/FirstPersonCharacter` (`GameplayStatics.GetPlayerCharacter` 0)))
  (set `self.PlayerCharacter` _asfirst_person_character))

(event `self.Box.OnComponentBeginOverlap`
  (params (OverlappedComponent :type "PrimitiveComponent Object Reference") (OtherActor :type "Actor Object Reference") (OtherComp :type "PrimitiveComponent Object Reference") (OtherBodyIndex :type Integer) (bFromSweep :type Boolean) (SweepResult :type "HitResult Structure (by ref)"))
  (bind _playercharacter (`self.PlayerCharacter`))
  (if (== OtherActor _playercharacter)
    (`self.DisableInput` _playercharacter (`GameplayStatics.GetPlayerController` 0))
    (`/Game/FirstPersonBP/FirstPersonCharacter.FadeOut` _playercharacter)
    (`KismetSystemLibrary.Delay` 0.75)
    (`GameplayStatics.OpenLevel` (`self.LevelName`))))

(fn `UserConstructionScript`)