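; Explosive barrel that loses health under laser hits, tinting its material by remaining health, and ignites at zero.
; Ignition spawns repeated flame emitters while a timeline flashes the color, then fires a radial impulse, explosion effects and destroys the actor.
; The player within range takes clamped, inverse-distance damage.
; Expanding the trigger sphere at detonation messages overlapping Explosion_Interface actors, so nearby barrels chain-react.
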(event `self.ReceiveBeginPlay`
  (bind _asfirst_person_character (cast `/Game/FirstPersonBP/FirstPersonCharacter` (`GameplayStatics.GetPlayerCharacter` 0)))
  (set `self.PlayerCharacter` _asfirst_person_character))

(event `IgniteBarrel`
  ;[1 1 1] Ignite barrel - flash barrel, impulse, damage player, destroy actor
  (set `self.Ignited` true)
  (bind (_direction _newtrack_0) (`Timeline|ColorChangeTimeline`)
    (:`Update`
      (bind _returnvalue (`PrimitiveComponent.CreateDynamicMaterialInstance` (`self.BarrelMesh`) 1 "/Game/Materials/Barrel_MAT.Barrel_MAT" "None"))
      (`MaterialInstanceDynamic.SetVectorParameterValue` _returnvalue "Color" (`KismetMathLibrary.LinearColorLerp` (struct :`R` 1.0 :`G` 0.8 :`A` 1.0) (struct :`R` 1.0 :`G` 1.0 :`B` 1.0 :`A` 1.0) _newtrack_0)))
    (:`Finished`
      (`SphereComponent.SetSphereRadius` (`self.NearbyObjectsTrigger`) 500.0 true)
      (`RadialForceComponent.FireImpulse` (`self.RadialForce`))
      (`self.DamagePlayer`)
      (`GameplayStatics.PlaySoundAtLocation` "/Game/Audio/Explosion_Audio.Explosion_Audio" (`self.K2_GetActorLocation`) (struct) 0.2 1.0 0.0 null null null) ; Play firing sound
      (`GameplayStatics.SpawnEmitterAtLocation` "/Game/Effects/Explosion_PS.Explosion_PS" (`SceneComponent.K2_GetComponentLocation` (`self.Cylinder`)))
      (`self.K2_DestroyActor`))))

(event `self.ReceiveTick`
  (params (DeltaSeconds :type "Float (single-precision)"))
  (if (`self.Ignited`)
    (`KismetSystemLibrary.Delay` 0.2)
    (`GameplayStatics.SpawnEmitterAtLocation` "/Game/Effects/Flame_PS.Flame_PS" (`SceneComponent.K2_GetComponentLocation` (`self.Cylinder`)))))

(event `DamagePlayer`
  (bind _returnvalue (`KismetMathLibrary.Vector_Distance` (`SceneComponent.K2_GetComponentLocation` (`self.Cylinder`)) (`SceneComponent.K2_GetComponentLocation` (`Character.CapsuleComponent` (`self.PlayerCharacter`)))))
  ;[1 1 1] Check if close enough to player
  (if (< _returnvalue 500.0)
    (`/Game/FirstPersonBP/FirstPersonCharacter.ChangePlayerHealth` (`self.PlayerCharacter`) (`KismetMathLibrary.FClamp` (/ -4000.0 _returnvalue) -30.0 0.0))))

(event `self.NearbyObjectsTrigger.OnComponentBeginOverlap`
  (params (OverlappedComponent :type "PrimitiveComponent Object Reference") (OtherActor :type "Actor Object Reference") (OtherComp :type "PrimitiveComponent Object Reference") (OtherBodyIndex :type Integer) (bFromSweep :type Boolean) (SweepResult :type "HitResult Structure (by ref)"))
  ;[1 1 1] Ignite any barrels nearby
  (if (`KismetSystemLibrary.DoesImplementInterface` OtherActor "/Game/Blueprints/Explosion_Interface.Explosion_Interface_C")
    (message `/Game/Blueprints/Explosion_Interface.ExplosionNearby` OtherActor)))

(event `/Game/Blueprints/Explosion_Interface.ExplosionNearby`
  (`self.IgniteBarrel`))

(event `/Game/Blueprints/Laserable_Interface.Laser`
  (params (Damage :type "Float (single-precision)"))
  ;[1 1 1] If being lasered
  (if (not (`self.Ignited`))
    (bind _output_get (set `self.Health` (- (`self.Health`) Damage)))
    (bind _returnvalue (`PrimitiveComponent.CreateDynamicMaterialInstance` (`self.BarrelMesh`) 1 "/Game/Materials/Barrel_MAT.Barrel_MAT" "None"))
    (`MaterialInstanceDynamic.SetVectorParameterValue` _returnvalue "Color" (`KismetMathLibrary.LinearColorLerp` (`KismetMathLibrary.MakeColor` 1.0 0.8 0.0 0.5) (`KismetMathLibrary.MakeColor` 0.875) (/ _output_get 100.0)))
    (if (<= (`self.Health`) 0.0)
      (`self.IgniteBarrel`))))

(fn `UserConstructionScript`)