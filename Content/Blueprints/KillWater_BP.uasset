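; KillWater_BP is a hazardous water volume that hurts the first-person player and weakens their jump while inside its box.
; Box overlap divides the character's jump velocity by 1.5 and starts a looping half-second timer, offset to begin damage immediately.
; Each timer call subtracts 20 health from the player character cached at BeginPlay.
; Leaving the box restores jump velocity and clears the timer.
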(event `self.ReceiveBeginPlay`
  (bind _asfirst_person_character (cast `/Game/FirstPersonBP/FirstPersonCharacter` (`GameplayStatics.GetPlayerCharacter` 0)))
  (set `self.PlayerCharacter` _asfirst_person_character))

(event `self.Box.OnComponentBeginOverlap`
  (params (OverlappedComponent :type "PrimitiveComponent Object Reference") (OtherActor :type "Actor Object Reference") (OtherComp :type "PrimitiveComponent Object Reference") (OtherBodyIndex :type Integer) (bFromSweep :type Boolean) (SweepResult :type "HitResult Structure (by ref)"))
  (bind _asfirst_person_character (cast `/Game/FirstPersonBP/FirstPersonCharacter` OtherActor))
  (bind _charactermovement (`Character.CharacterMovement` _asfirst_person_character))
  (set `CharacterMovementComponent.JumpZVelocity` (/ (`CharacterMovementComponent.JumpZVelocity` _charactermovement) 1.5) _charactermovement)
  (`KismetSystemLibrary.K2_SetTimer` null "DamagePlayer" 0.5 true -0.5))

(event `self.Box.OnComponentEndOverlap`
  (params (OverlappedComponent :type "PrimitiveComponent Object Reference") (OtherActor :type "Actor Object Reference") (OtherComp :type "PrimitiveComponent Object Reference") (OtherBodyIndex :type Integer))
  (bind _asfirst_person_character (cast `/Game/FirstPersonBP/FirstPersonCharacter` OtherActor))
  (bind _charactermovement (`Character.CharacterMovement` _asfirst_person_character))
  (set `CharacterMovementComponent.JumpZVelocity` (* (`CharacterMovementComponent.JumpZVelocity` _charactermovement) 1.5) _charactermovement)
  (`KismetSystemLibrary.K2_ClearTimer` null "DamagePlayer"))

(event `DamagePlayer`
  (`/Game/FirstPersonBP/FirstPersonCharacter.ChangePlayerHealth` (`self.PlayerCharacter`) -20.0))

(fn `UserConstructionScript`)